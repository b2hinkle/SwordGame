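; Garage door actor for the residential house that opens through its animation Blueprint when its trigger is overlapped.
; BeginPlay caches AnimBP_DoorGarage and checks the level name, then overlaps drive that anim instance's PlayerNear flag.
; Outside EnemyHouse, only the player character's capsule sets the flag, playing audio once, and nothing clears it.
; In EnemyHouse, any overlap sets it silently and any end overlap clears it.
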(event OnComponentBeginOverlap(Trigger)
  (params (OverlappedComponent :type Primitive%20Component%20Object%20Reference) (OtherActor :type Actor%20Object%20Reference) (OtherComp :type Primitive%20Component%20Object%20Reference) (OtherBodyIndex :type Integer) (bFromSweep :type Boolean) (SweepResult :type Hit%20Result%20Structure%20%28by%20ref%29))
  (Utilities|Casting|CastToAnimBP_DoorGarage (Components|SkeletalMesh|GetAnimInstance (Variables|Default|GetGarage_door)))
  (if (Variables|Default|GetIsNotPartyMap)
    (bind _asthird_person_character (Utilities|Casting|CastToThirdPersonCharacter OtherActor))
    (if (== (Variables|/Script/Engine.Character|GetCapsuleComponent _asthird_person_character) OtherComp)
      (if (not (Variables|/Game/HQ_ResidentialHouse/Meshes/DoorGarage/AnimBP_DoorGarage.AnimBP_DoorGarage_C|GetPlayerNear (Variables|Default|GetDoorAnimBP)))
        (Variables|/Game/HQ_ResidentialHouse/Meshes/DoorGarage/AnimBP_DoorGarage.AnimBP_DoorGarage_C|SetPlayerNear (Variables|Default|GetDoorAnimBP) true)
        (Components|Activation|Activate (Variables|Default|GetAudio) true)))
    (else
      (Variables|/Game/HQ_ResidentialHouse/Meshes/DoorGarage/AnimBP_DoorGarage.AnimBP_DoorGarage_C|SetPlayerNear (Variables|Default|GetDoorAnimBP) true))))

(event OnComponentEndOverlap(Trigger)
  (params (OverlappedComponent :type Primitive%20Component%20Object%20Reference) (OtherActor :type Actor%20Object%20Reference) (OtherComp :type Primitive%20Component%20Object%20Reference) (OtherBodyIndex :type Integer))
  (Utilities|Casting|CastToAnimBP_DoorGarage (Components|SkeletalMesh|GetAnimInstance (Variables|Default|GetGarage_door)))
  (if (not (Variables|Default|GetIsNotPartyMap))
    (Variables|/Game/HQ_ResidentialHouse/Meshes/DoorGarage/AnimBP_DoorGarage.AnimBP_DoorGarage_C|SetPlayerNear (Variables|Default|GetDoorAnimBP) false)))

(event EventBeginPlay
  (bind _asanim_bp_door_garage (Utilities|Casting|CastToAnimBP_DoorGarage (Components|SkeletalMesh|GetAnimInstance (Variables|Default|GetGarage_door))))
  (Variables|Default|SetDoorAnimBP _asanim_bp_door_garage)
  (bind _returnvalue (Game|GetCurrentLevelName true))
  (if (Utilities|Enum|Equal(Enum) _returnvalue "EnemyHouse")
    (Variables|Default|SetisNotPartyMap false)
    (else
      (Variables|Default|SetisNotPartyMap true))))

(fn ConstructionScript)