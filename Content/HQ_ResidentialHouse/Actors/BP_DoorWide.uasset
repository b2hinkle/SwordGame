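; BP_DoorWide is a wide door actor that reacts to the player approaching, driven by an animation Blueprint.
; On BeginPlay it caches the door mesh's AnimBP_DoorWide instance and sets IsNotPartyMap to false only in the EnemyHouse level.
; Its Trigger sets PlayerNear on that instance when a ThirdPersonCharacter capsule enters, and clears it when the character's overlap ends.
; IsNotPartyMap is not read in this Blueprint's graphs.
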(event OnComponentEndOverlap(Trigger)
  (params (OverlappedComponent :type Primitive%20Component%20Object%20Reference) (OtherActor :type Actor%20Object%20Reference) (OtherComp :type Primitive%20Component%20Object%20Reference) (OtherBodyIndex :type Integer))
  (if (== (Utilities|GetClass OtherActor) "/Game/Player/ThirdPersonCharacter.ThirdPersonCharacter_C")
    (Variables|/Game/HQ_ResidentialHouse/Meshes/DoorWide/AnimBP_DoorWide.AnimBP_DoorWide_C|SetPlayerNear (Variables|Default|GetNewVar_0) false)))

(event OnComponentBeginOverlap(Trigger)
  (params (OverlappedComponent :type Primitive%20Component%20Object%20Reference) (OtherActor :type Actor%20Object%20Reference) (OtherComp :type Primitive%20Component%20Object%20Reference) (OtherBodyIndex :type Integer) (bFromSweep :type Boolean) (SweepResult :type Hit%20Result%20Structure%20%28by%20ref%29))
  (if (== (Utilities|GetClass OtherActor) "/Game/Player/ThirdPersonCharacter.ThirdPersonCharacter_C")
    (if (== (Utilities|GetClass OtherComp) "/Script/Engine.CapsuleComponent")
      (Variables|/Game/HQ_ResidentialHouse/Meshes/DoorWide/AnimBP_DoorWide.AnimBP_DoorWide_C|SetPlayerNear (Variables|Default|GetNewVar_0) true))))

(event EventBeginPlay
  (bind _asanim_bp_door_wide (Utilities|Casting|CastToAnimBP_DoorWide (Components|SkeletalMesh|GetAnimInstance (Variables|Default|GetDoor_wide))))
  (Variables|Default|SetNewVar_0 _asanim_bp_door_wide)
  (bind _returnvalue (Game|GetCurrentLevelName true))
  (if (Utilities|Enum|Equal(Enum) _returnvalue "EnemyHouse")
    (Variables|Default|SetisNotPartyMap false)
    (else
      (Variables|Default|SetisNotPartyMap true))))

(fn ConstructionScript)