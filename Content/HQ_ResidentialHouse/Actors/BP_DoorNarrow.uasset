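; BP_DoorNarrow is a narrow door actor that reacts to the player character's proximity.
; On BeginPlay it caches the door mesh's AnimBPDoorNarrow instance, then sets IsNotPartyMap false only on the EnemyHouse level; this graph never reads that flag.
; Trigger overlaps with a ThirdPersonCharacter's capsule toggle PlayerNear on the anim instance, leaving door motion to the Animation Blueprint.
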(event OnComponentEndOverlap(Trigger)
  (params (OverlappedComponent :type Primitive%20Component%20Object%20Reference) (OtherActor :type Actor%20Object%20Reference) (OtherComp :type Primitive%20Component%20Object%20Reference) (OtherBodyIndex :type Integer))
  (bind _asthird_person_character (Utilities|Casting|CastToThirdPersonCharacter OtherActor))
  (if (== (Variables|/Script/Engine.Character|GetCapsuleComponent _asthird_person_character) OtherComp)
    (Variables|/Game/HQ_ResidentialHouse/Meshes/DoorNarrow/AnimBPDoorNarrow.AnimBPDoorNarrow_C|SetPlayerNear (Variables|Default|GetNewVar_0) false)))

(event OnComponentBeginOverlap(Trigger)
  (params (OverlappedComponent :type Primitive%20Component%20Object%20Reference) (OtherActor :type Actor%20Object%20Reference) (OtherComp :type Primitive%20Component%20Object%20Reference) (OtherBodyIndex :type Integer) (bFromSweep :type Boolean) (SweepResult :type Hit%20Result%20Structure%20%28by%20ref%29))
  (bind _asthird_person_character (Utilities|Casting|CastToThirdPersonCharacter OtherActor))
  (if (== (Variables|/Script/Engine.Character|GetCapsuleComponent _asthird_person_character) OtherComp)
    (Variables|/Game/HQ_ResidentialHouse/Meshes/DoorNarrow/AnimBPDoorNarrow.AnimBPDoorNarrow_C|SetPlayerNear (Variables|Default|GetNewVar_0) true)))

(event EventBeginPlay
  (bind _asanim_bpdoor_narrow (Utilities|Casting|CastToAnimBPDoorNarrow (Components|SkeletalMesh|GetAnimInstance (Variables|Default|GetDoor_narrow))))
  (Variables|Default|SetNewVar_0 _asanim_bpdoor_narrow)
  (bind _returnvalue (Game|GetCurrentLevelName true))
  (if (Utilities|Enum|Equal(Enum) _returnvalue "EnemyHouse")
    (Variables|Default|SetisNotPartyMap false)
    (else
      (Variables|Default|SetisNotPartyMap true))))

(fn ConstructionScript)