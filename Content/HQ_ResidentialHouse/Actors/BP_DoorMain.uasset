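; BP_DoorMain is the residential house's main door actor, which reacts to the player approaching and leaving.
; Its trigger overlaps, filtered to the ThirdPersonCharacter's capsule, toggle PlayerNear on the cached door animation blueprint.
; Entering also plays an attenuated opening sound at the door.
; At BeginPlay it sets IsNotPartyMap by checking whether the level is EnemyHouse, though this graph never reads that flag.
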(event OnComponentEndOverlap(Trigger)
  (params (OverlappedComponent :type Primitive%20Component%20Object%20Reference) (OtherActor :type Actor%20Object%20Reference) (OtherComp :type Primitive%20Component%20Object%20Reference) (OtherBodyIndex :type Integer))
  (bind _asthird_person_character (Utilities|Casting|CastToThirdPersonCharacter OtherActor))
  (if (== (Variables|/Script/Engine.Character|GetCapsuleComponent _asthird_person_character) OtherComp)
    (Variables|/Game/HQ_ResidentialHouse/Meshes/DoorMain/AnimBPDoorMain.AnimBPDoorMain_C|SetPlayerNear (Variables|Default|Getabim1) false)))

(event OnComponentBeginOverlap(Trigger)
  (params (OverlappedComponent :type Primitive%20Component%20Object%20Reference) (OtherActor :type Actor%20Object%20Reference) (OtherComp :type Primitive%20Component%20Object%20Reference) (OtherBodyIndex :type Integer) (bFromSweep :type Boolean) (SweepResult :type Hit%20Result%20Structure%20%28by%20ref%29))
  (bind _asthird_person_character (Utilities|Casting|CastToThirdPersonCharacter OtherActor))
  (if (== (Variables|/Script/Engine.Character|GetCapsuleComponent _asthird_person_character) OtherComp)
    (Variables|/Game/HQ_ResidentialHouse/Meshes/DoorMain/AnimBPDoorMain.AnimBPDoorMain_C|SetPlayerNear (Variables|Default|Getabim1) true)
    (Audio|PlaySoundatLocation "/Game/sounds/DoorOpen.DoorOpen" (Transformation|GetActorLocation) "0, 0, 0" 0.6 1.0 0.0 "/Game/sounds/DoorCreek.DoorCreek" 0 0 0)))

(event EventBeginPlay
  (bind _asanim_bpdoor_main (Utilities|Casting|CastToAnimBPDoorMain (Components|SkeletalMesh|GetAnimInstance (Variables|Default|GetDoor_main))))
  (Variables|Default|Setabim1 _asanim_bpdoor_main)
  (bind _returnvalue (Game|GetCurrentLevelName true))
  (if (Utilities|Enum|Equal(Enum) _returnvalue "EnemyHouse")
    (Variables|Default|SetisNotPartyMap false)
    (else
      (Variables|Default|SetisNotPartyMap true))))

(fn ConstructionScript)