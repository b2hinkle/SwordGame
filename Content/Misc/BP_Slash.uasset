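; BP_Slash is the short-lived slash actor of a heavy swing, acting as both hitbox and visual effect.
; On authority it overlaps its mesh against character pawns once at spawn, hits one chosen living player, then self-destructs after a generous delay.
; If that hit kills, it multicasts a slash-hit event through the instigator.
; Remote instances only timestamp a dynamic material instance to drive the slash visual.
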(event Custom|PerformOverlapTestAndApplyDmg
  (bind _returnvalue (Game|GetInstigator))
  (bind _staticmesh (Variables|Default|GetStaticMesh))
  (bind _outactors (Collision|ComponentOverlapActors _staticmesh (Transformation|GetWorldTransform _staticmesh) (Utilities|Array|MakeArray "ObjectTypeQuery3") "/Script/Engine.Character" (Utilities|Array|MakeArray _returnvalue self)))
  (bind _asthird_person_character (Utilities|Casting|CastToThirdPersonCharacter _returnvalue))
  (bind _chosentpc (CallFunction|ChoosePlayerfromHeavySwingOverlapResults _outactors _asthird_person_character))
  (if (not (Default|IsDead _chosentpc))
    (CallFunction|HandleTPCThatWasHeavyHitted _chosentpc _asthird_person_character)
    (if (Default|IsDead _chosentpc)
      (Default|MultionSlashHitPlayer _asthird_person_character self))))

(event EventBeginPlay
  (Networking|SwitchHasAuthority
    (:Authority
      (CallFunction|PerformOverlapTestandApplyDmg)
      ;[0.15 0.15 0.15 0.5 10] Note: Arbitrary duration but we know it shouldn't be visible after this amt.
      (Utilities|FlowControl|Delay 8.0)
      (Actor|DestroyActor))
    (:Remote
      (bind _returnvalue (Rendering|Material|CreateDynamicMaterialInstance (Variables|Default|GetStaticMesh) 0 "/Game/Meshes/Slashes/M_Slash.M_Slash" "None" :!class /Script/Engine.PrimitiveComponent))
      (bind _output_get (Variables|Default|SetDynamicMatInst _returnvalue))
      (Rendering|Material|SetScalarParameterValue _output_get "TimeStamp" (Utilities|Time|GetTimeSeconds) :!class /Script/Engine.MaterialInstanceDynamic))))

(fn ConstructionScript)