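; Safe room actor that can be shown or hidden and displays a countdown taken from the RotatingDoor's fast-spin timer.
; MultiEnable reveals its components, restores mesh collision, resets the countdown and activates the level's wind sound on clients.
; MultiDisable has the server move overlapping characters to a fixed location, then hides components and disables mesh collision.
; Tick decrements the timer and writes the rounded value to a text render.
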(event Custom|MultiEnable
  (bind _windsound (Variables|Default|GetWindSound))
  (Networking|SwitchHasAuthority
    (:Authority
      _)
    (:Remote
      (Utilities|IsValid _windsound
        (:Is%20Valid
          (Components|Activation|Activate (Variables|/Script/Engine.AmbientSound|GetAudioComponent _windsound) true))
        (:Is%20Not%20Valid
          _))))
  (for _array_element (Actor|GetComponentsByClass "/Script/Engine.ActorComponent")
    (bind _asscene_component (Utilities|Casting|CastToSceneComponent _array_element))
    (Development|SetHiddeninGame _asscene_component false false)
    (bind _asstatic_mesh_component (Utilities|Casting|CastToStaticMeshComponent _asscene_component))
    (Collision|SetCollisionEnabled _asstatic_mesh_component "QueryAndPhysics"))
  (Variables|Default|SetTimer (Variables|/Game/Door/RotatingDoor.RotatingDoor_C|Getspinfasttimer (Variables|Default|GetRotatingDoor))))

(event Custom|MultiDisable
  (Networking|SwitchHasAuthority
    (:Authority
      (for _array_element (Collision|GetOverlappingActors (Variables|Default|GetBox) "/Game/Player/ThirdPersonCharacter.ThirdPersonCharacter_C" :!class /Script/Engine.PrimitiveComponent)
        (Transformation|SetActorLocation _array_element "0,247.000000,227.000000" false false)))
    (:Remote
      _))
  (for _array_element_2 (Actor|GetComponentsByClass "/Script/Engine.ActorComponent")
    (bind _asscene_component (Utilities|Casting|CastToSceneComponent _array_element_2))
    (Development|SetHiddeninGame _asscene_component true false)
    (bind _asstatic_mesh_component (Utilities|Casting|CastToStaticMeshComponent _asscene_component))
    (Collision|SetCollisionEnabled _asstatic_mesh_component "NoCollision")))

(event EventBeginPlay
  (Networking|SwitchHasAuthority
    (:Authority
      (bind _outactors (Actor|GetAllActorsOfClass "/Game/Door/RotatingDoor.RotatingDoor_C"))
      (for _array_element _outactors
        (Utilities|IsValid _array_element
          (:Is%20Valid
            (Variables|Default|SetRotatingDoor _array_element))))
      (Variables|Default|SetTimer (Variables|/Game/Door/RotatingDoor.RotatingDoor_C|Getspinfasttimer (Variables|Default|GetRotatingDoor))))
    (:Remote
      (bind _outactors_2 (Actor|GetAllActorsOfClass "/Game/Door/SafeRoomWind_Blueprint.SafeRoomWind_Blueprint_C"))
      (for _array_element_2 _outactors_2
        (Variables|Default|SetWindSound _array_element_2)))))

(event EventTick
  (params (DeltaSeconds :type Float%20%28single-precision%29))
  (bind _newtextrendercomponent1 (Variables|Default|GetNewTextRenderComponent1))
  (bind _output_get (Variables|Default|SetTimer (- (Variables|Default|GetTimer) DeltaSeconds)))
  (Utilities|IsValid _newtextrendercomponent1
    (:Is%20Valid
      (Rendering|Components|TextRender|SetText _newtextrendercomponent1 (Utilities|Text|ToText(Integer) (Math|Float|Round _output_get))))))

(fn ConstructionScript)