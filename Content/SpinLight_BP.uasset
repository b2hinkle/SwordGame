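; SpinLight_BP is a light fixture Blueprint that switches between a lit and an unlit state through spin-speed events.
; OnSpinFast unhides its two spotlights in game and swaps the static mesh material to Red_2.
; OnSpinSlow hides both spotlights and sets the material to Red.
; The graph holds no rotation logic or callers for these events, and the construction script is empty.
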(event Custom|OnSpinFast
  (Development|SetHiddeninGame (Variables|Default|GetSpotLight) false false)
  (Development|SetHiddeninGame (Variables|Default|GetSpotLight1) false false)
  (Rendering|Material|SetMaterial (Variables|Default|GetStaticMesh) 0 "/Game/Meshes/Controller/Red_2.Red_2"))

(event Custom|OnSpinSlow
  (Development|SetHiddeninGame (Variables|Default|GetSpotLight) true false)
  (Development|SetHiddeninGame (Variables|Default|GetSpotLight1) true false)
  (Rendering|Material|SetMaterial (Variables|Default|GetStaticMesh) 0 "/Game/Meshes/Controller/Red.Red"))

(fn ConstructionScript)