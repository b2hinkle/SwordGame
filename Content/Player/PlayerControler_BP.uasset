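; Player controller for a multiplayer game, handling a seeded garage-door dance cutscene, match timer, ready counts and character spawning at random starts.
; BeginPlay applies high graphics settings, adds a compressor and binds the player menu toggle, while key 9 flips quality presets.
; Handle functions forward travel, restart, ability and mod commands to the controlled ThirdPersonCharacter, some gated by ModsAllowed.
; The submitted-link multicast ends at an empty switch, leaving browser music code disconnected.
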(event Custom|SpawnThirdPersonCharacter
  (bind _outactors (Actor|GetAllActorsOfClass "/Script/Engine.PlayerStart"))
  (Game|SpawnActorfromClass "/Game/Player/ThirdPersonCharacter.ThirdPersonCharacter_C" (Math|Transform|MakeTransform (.location (Transformation|GetActorTransform (Utilities|Array|Get(acopy) _outactors (Math|Random|RandomIntegerinRange 0 (- (Utilities|Array|Length _outactors) 1))))) (Math|Rotator|MakeRotator (.Roll (Math|Rotator|BreakRotator (.rotation (Transformation|GetActorTransform (Utilities|Array|Get(acopy) _outactors (Math|Random|RandomIntegerinRange 0 (- (Utilities|Array|Length _outactors) 1))))))) (.Pitch (Math|Rotator|BreakRotator (.rotation (Transformation|GetActorTransform (Utilities|Array|Get(acopy) _outactors (Math|Random|RandomIntegerinRange 0 (- (Utilities|Array|Length _outactors) 1))))))) (.Yaw (Math|Rotator|BreakRotator (.rotation (Transformation|GetActorTransform (Utilities|Array|Get(acopy) _outactors (Math|Random|RandomIntegerinRange 0 (- (Utilities|Array|Length _outactors) 1)))))))) (.scale (Transformation|GetActorTransform (Utilities|Array|Get(acopy) _outactors (Math|Random|RandomIntegerinRange 0 (- (Utilities|Array|Length _outactors) 1)))))) "AdjustIfPossibleButAlwaysSpawn" "MultiplyWithRoot" 0 0))

(event Custom|ServerDecrementPlayersReady
  (bind _ashouse_e_gm (Utilities|Casting|CastToHouseE_GM (Game|GetGameMode)))
  (Math|Integer|DecrementInt (Variables|/Game/HouseE_GM.HouseE_GM_C|GetNumOfPlayersReady _ashouse_e_gm)))

(event Custom|ClientResponseToStartingCutscene
  (params (ServerGeneratedSeed :type Integer))
  (bind _starttime (CallFunction|GetRandomStartTimeforNonSambaDancingAnim(0-9Chance) ServerGeneratedSeed))
  (Development|PrintString (Utilities|String|ToString(Float) _starttime) true true (Math|Conversions|ToLinearColor(Float) _starttime) 0.2)
  (bind _outactors (Actor|GetAllActorsOfClass "/Game/Enemy/Enemy.Enemy_C"))
  (bind _output_get (Variables|Default|SetenemyArray _outactors))
  (for _array_element _output_get
    (if (and (Utilities|Enum|NotEqual(Enum) "Belly_Dance" (Utilities|GetDisplayName (.AnimToPlay (Utilities|Struct|BreakSingleAnimationPlayData (Variables|/Script/Engine.SkeletalMeshComponent|GetAnimationData (Variables|/Script/Engine.Character|GetMesh _array_element)))))) (and (Utilities|Enum|NotEqual(Enum) "TalkingPhone" (Utilities|GetDisplayName (.AnimToPlay (Utilities|Struct|BreakSingleAnimationPlayData (Variables|/Script/Engine.SkeletalMeshComponent|GetAnimationData (Variables|/Script/Engine.Character|GetMesh _array_element)))))) (and (Utilities|Enum|NotEqual(Enum) "Talking__2_" (Utilities|GetDisplayName (.AnimToPlay (Utilities|Struct|BreakSingleAnimationPlayData (Variables|/Script/Engine.SkeletalMeshComponent|GetAnimationData (Variables|/Script/Engine.Character|GetMesh _array_element)))))) (Utilities|Enum|NotEqual(Enum) "Talking" (Utilities|GetDisplayName (.AnimToPlay (Utilities|Struct|BreakSingleAnimationPlayData (Variables|/Script/Engine.SkeletalMeshComponent|GetAnimationData (Variables|/Script/Engine.Character|GetMesh _array_element)))))))))
      (Components|Animation|PlayAnimation (Variables|/Script/Engine.Character|GetMesh _array_element) "/Game/EnemyModel/enemy1/Samba_Dancing_Anim.Samba_Dancing_Anim" true)
      (Components|Activation|Activate (Variables|/Game/Enemy/Enemy.Enemy_C|GetBears _array_element) true)
      (bind _outactors_2 (Actor|GetAllActorsOfClass "/Script/Engine.AmbientSound"))
      (for _array_element_2 _outactors_2
        (Components|Activation|Activate (Variables|/Script/Engine.AmbientSound|GetAudioComponent _array_element_2) true)
        (Utilities|FlowControl|Delay 24.0)
        (bind _outactors_3 (Actor|GetAllActorsOfClass "/Game/CutsceneGarageDoor.CutsceneGarageDoor_C"))
        (for _array_element_3 _outactors_3
          (Default|StartGaragedroor _array_element_3)))
      (elif (Utilities|Enum|Equal(Enum) (Utilities|GetDisplayName (.AnimToPlay (Utilities|Struct|BreakSingleAnimationPlayData (Variables|/Script/Engine.SkeletalMeshComponent|GetAnimationData (Variables|/Script/Engine.Character|GetMesh _array_element))))) "TalkingPhone")
        (Components|Animation|SetPosition (Variables|/Script/Engine.Character|GetMesh _array_element) 3.0 false)
        (else
          (Components|Animation|SetPosition (Variables|/Script/Engine.Character|GetMesh _array_element) _starttime false)))))
  (Class|PlayerController|SetAudioListenerOverride 0 "0, 0,-1350.000000" "0, 0, 0")
  (Utilities|FlowControl|Delay 7.2)
  (Class|PlayerController|ClearAudioListenerOverride))

(event Custom|CallClientResponseToStartingCutsceneWithRandomGeneratedSeed
  (CallFunction|ClientResponsetoStartingCutscene (Math|Random|RandomIntegerinRange 0 9)))

(event Custom|InputProcessorPlayerMenuInputPress
  (bind _isa (Utilities|FlowControl|FlipFlop)
    (:A
      _)
    (:B
      _))
  (CallFunction|EnablePlayerMenuWidget _isa))

(event Custom|EnablePlayerMenuWidget
  (params (ShouldEnable :type Boolean))
  (bind _self self)
  (if ShouldEnable
    (bind _returnvalue (UserInterface|CreateWidget "/Game/UI/WBP_PlayerMenu.WBP_PlayerMenu_C" _self))
    (bind _output_get (Variables|Default|SetPlayerMenuWidget _returnvalue))
    (UserInterface|Viewport|AddtoPlayerScreen _output_get)
    (Input|SetInputModeUIOnly _self _output_get "DoNotLock" true)
    (Variables|/Script/Engine.PlayerController|SetbShowMouseCursor _self true)
    (else
      (Widget|RemovefromParent (Variables|Default|GetPlayerMenuWidget))
      (Input|SetInputModeGameOnly _self false)
      (Variables|/Script/Engine.PlayerController|SetbShowMouseCursor _self false))))

(event Custom|ServerIncrementPlayerReady
  (bind _ashouse_e_gm (Utilities|Casting|CastToHouseE_GM (Game|GetGameMode)))
  (bind _result (Math|Integer|IncrementInt (Variables|/Game/HouseE_GM.HouseE_GM_C|GetNumOfPlayersReady _ashouse_e_gm))
    (:%20%20
      (Development|PrintString (Utilities|String|Append (Utilities|String|ToString(Integer) _result) " Player(s) Ready") true true "(R=1.000000,G=0.000000,B=0.398021,A=1.000000)" 3.0))))

(event Custom|StopTimer
  (if (Pawn|IsLocalPlayerController)
    (Variables|/Game/UI/Timer.Timer_C|SetTimerStarted (Variables|Default|GetClientTimer) false)
    (Audio|PlaySound2D "/Game/sounds/PutSwordAway.PutSwordAway" 2e+01 1.0 0.0 0 0)))

(event Custom|PlayerSubmittedLink
  (CallFunction|ServerPlayerSubmittedLink (Variables|Default|Geturl)))

(event Custom|ServerCallGameMode'sStartGame
  (bind _ashouse_e_gm (Utilities|Casting|CastToHouseE_GM (Game|GetGameMode)))
  (Default|StartGame _ashouse_e_gm))

(event Custom|ClearMenuAndSetInputmodeToGame
  (Viewport|RemoveAllWidgets)
  (Input|SetInputModeGameOnly self false))

(event Custom|MultiPlayersStartedPlaying
  (Networking|SwitchHasAuthority
    (:Remote
      (Audio|PlaySound2D "/Game/sounds/Spawnt.Spawnt" 3.0 1.0 0.0 0 0)
      (if (Pawn|IsLocalPlayerController)
        (bind _returnvalue (UserInterface|CreateWidget "/Game/UI/Timer.Timer_C" self))
        (bind _output_get (Variables|Default|SetClientTimer _returnvalue))
        (UserInterface|Viewport|AddtoViewport _output_get 0)
        (Variables|/Game/UI/Timer.Timer_C|SetTimerStarted _output_get true)
        (bind _asthird_person_character (Utilities|Casting|CastToThirdPersonCharacter (Pawn|GetControlledPawn)))
        (Class|PlayerController|SetAudioListenerOverride (Variables|/Script/Engine.Character|GetCapsuleComponent _asthird_person_character) "0, 0, 0" "0, 0, 0")))))

(event Custom|ServerPlayerSubmittedLink
  (params (url :type String))
  (CallFunction|MultiPlayerSubmittedLink url))

(event Custom|MultiPlayerSubmittedLink
  (params (url :type String))
  (Networking|SwitchHasAuthority))

(event EventEndPlay
  (params (EndPlayReason :type EEndPlayReason%20Enum :default "Destroyed"))
  (Class|SwordGameBlueprintFunctionLibrary|OnPlayerMenuInputPressRemovebyCtxObj self))

(event EventBeginPlay
  (if (Pawn|IsLocalPlayerController)
    (Class|AudioMixerBlueprintLibrary|SetSubmixEffectChainOverride "/Engine/EngineSounds/Submixes/MasterSubmixDefault.MasterSubmixDefault" (Utilities|Array|MakeArray "/Game/Effects/compressor.compressor") 0.0)
    (Class|SwordGameBlueprintFunctionLibrary|ExecuteonPlayerMenuInputPress self (delegate Custom|InputProcessorPlayerMenuInputPress)))
  (bind _returnvalue (Game|GetCurrentLevelName true))
  (Variables|Default|SetLevelName _returnvalue)
  (Networking|SwitchHasAuthority
    (:Authority
      _)
    (:Remote
      (bind _asninja_game_gi (Utilities|Casting|CastToNinjaGame_GI (Game|GetGameInstance))
        (:then
          (Variables|/Game/NinjaGame_GI.NinjaGame_GI_C|SetLastJoinedIP _asninja_game_gi (Class|SwordGamePlayerController|GetNetworkURL)))
        (:CastFailed
          _))))
  (bind _returnvalue_2 (UserInterface|CreateWidget "/Game/UI/GraphicsQuality.GraphicsQuality_C"))
  (Utilities|IsValid _returnvalue_2
    (:Is%20Valid
      (UserInterface|Viewport|AddtoViewport _returnvalue_2 0))
    (:Is%20Not%20Valid
      _))
  (bind _returnvalue_3 (Settings|GetGameUserSettings))
  (Class|GameUserSettings|ApplySettings _returnvalue_3 false)
  (Class|GameUserSettings|SetResolutionScaleValueEx _returnvalue_3 1e+02)
  (Class|GameUserSettings|SetViewDistanceQuality _returnvalue_3)
  (Class|GameUserSettings|SetAntiAliasingQuality _returnvalue_3 3)
  (Class|GameUserSettings|SetPostProcessingQuality _returnvalue_3 3)
  (Class|GameUserSettings|SetShadowQuality _returnvalue_3 3)
  (Class|GameUserSettings|SetTextureQuality _returnvalue_3 3)
  (Class|GameUserSettings|SetVisualEffectQuality _returnvalue_3 3)
  (Class|GameUserSettings|SetFoliageQuality _returnvalue_3)
  (Class|GameUserSettings|ApplySettings _returnvalue_3 false))

(event Input|KeyboardEvents|9
  (params (Key :type Key%20Structure :default "None"))
  (:Pressed
    (Utilities|FlowControl|FlipFlop
      (:A
        (Development|PrintString "Graphics switched to low" true false "(R=1.000000,G=0.000000,B=0.282353,A=1.000000)" 4.0)
        (bind _returnvalue (Settings|GetGameUserSettings))
        (Class|GameUserSettings|SetResolutionScaleValueEx _returnvalue 8e+01)
        (Class|GameUserSettings|SetViewDistanceQuality _returnvalue)
        (Class|GameUserSettings|SetAntiAliasingQuality _returnvalue)
        (Class|GameUserSettings|SetPostProcessingQuality _returnvalue 3)
        (Class|GameUserSettings|SetShadowQuality _returnvalue 1)
        (Class|GameUserSettings|SetTextureQuality _returnvalue 3)
        (Class|GameUserSettings|SetVisualEffectQuality _returnvalue 3)
        (Class|GameUserSettings|SetFoliageQuality _returnvalue)
        (Class|GameUserSettings|ApplySettings _returnvalue false)
        (Audio|PlaySound2D "/Game/sounds/SFX/UI/Button/ButtonClickSFX.ButtonClickSFX" 1.0 1.0 0.0 0 0))
      (:B
        (Development|PrintString "Graphics switched to high" true false "(R=1.000000,G=0.000000,B=0.795438,A=1.000000)" 4.0)
        (bind _returnvalue_2 (Settings|GetGameUserSettings))
        (Class|GameUserSettings|SetResolutionScaleValueEx _returnvalue_2 1e+02)
        (Class|GameUserSettings|SetViewDistanceQuality _returnvalue_2)
        (Class|GameUserSettings|SetAntiAliasingQuality _returnvalue_2 3)
        (Class|GameUserSettings|SetPostProcessingQuality _returnvalue_2 3)
        (Class|GameUserSettings|SetShadowQuality _returnvalue_2 3)
        (Class|GameUserSettings|SetTextureQuality _returnvalue_2 3)
        (Class|GameUserSettings|SetVisualEffectQuality _returnvalue_2 3)
        (Class|GameUserSettings|SetFoliageQuality _returnvalue_2)
        (Class|GameUserSettings|ApplySettings _returnvalue_2 false)
        (Audio|PlaySound2D "/Game/sounds/SFX/UI/Button/ButtonClickSFX.ButtonClickSFX" 1.0 1.0 0.0 0 0)))))

(fn ConstructionScript
  (Pawn|SetControlRotation (Math|Rotator|MakeRotator 0.0 0.0 -9e+01)))

(fn OnRepBClientRepPossess)

(fn HandleTraveltoWorld
  (params (mapName :type Name%20%28by%20ref%29 :default "None"))
  (bind _asthird_person_character (Utilities|Casting|CastToThirdPersonCharacter (Pawn|GetControlledPawn)))
  (Default|ServerChangeServerMap _asthird_person_character (Utilities|String|ToString(Name) mapName)))

(fn HandleRestartWorld
  (bind _asthird_person_character (Utilities|Casting|CastToThirdPersonCharacter (Pawn|GetControlledPawn)))
  (Default|ServerRestartServer _asthird_person_character))

(fn HandleForceReconnectAllPlayers
  (bind _asthird_person_character (Utilities|Casting|CastToThirdPersonCharacter (Pawn|GetControlledPawn)))
  (Default|ServerForceReconnectEachPlayer _asthird_person_character))

(fn HandleBallz
  (params (howMany :type Integer))
  (bind _asthird_person_character (Utilities|Casting|CastToThirdPersonCharacter (Pawn|GetControlledPawn)))
  (if (Variables|/Game/Player/ThirdPersonCharacter.ThirdPersonCharacter_C|GetbModsAllowed _asthird_person_character)
    (Default|ServerBallz _asthird_person_character howMany)))

(fn HandleClearObjects
  (bind _asthird_person_character (Utilities|Casting|CastToThirdPersonCharacter (Pawn|GetControlledPawn)))
  (if (Variables|/Game/Player/ThirdPersonCharacter.ThirdPersonCharacter_C|GetbModsAllowed _asthird_person_character)
    (Default|ServerClearObjs _asthird_person_character)))

(fn HandleEnableFriendlyFireforRandomPlayer
  (bind _asthird_person_character (Utilities|Casting|CastToThirdPersonCharacter (Pawn|GetControlledPawn)))
  (Default|SelectRandomPlayertobeIt _asthird_person_character))

(fn HandleGiveChargeAbility
  (bind _asthird_person_character (Utilities|Casting|CastToThirdPersonCharacter (Pawn|GetControlledPawn)))
  (Default|ServerGiveCharge _asthird_person_character))

(fn HandleGiveMineAbility
  (bind _asthird_person_character (Utilities|Casting|CastToThirdPersonCharacter (Pawn|GetControlledPawn)))
  (Default|ServerGiveMines _asthird_person_character))

(fn HandleGiveTeleportAbility
  (bind _asthird_person_character (Utilities|Casting|CastToThirdPersonCharacter (Pawn|GetControlledPawn)))
  (Default|ServerGiveTeleoprt _asthird_person_character))

(fn HandleLaunchSelf
  (params (force :type Float%20%28single-precision%29))
  (bind _asthird_person_character (Utilities|Casting|CastToThirdPersonCharacter (Pawn|GetControlledPawn)))
  (if (Variables|/Game/Player/ThirdPersonCharacter.ThirdPersonCharacter_C|GetbModsAllowed _asthird_person_character)
    (Default|ServerAddForce _asthird_person_character force)))

(fn HandleMrIncredi1
  (bind _asthird_person_character (Utilities|Casting|CastToThirdPersonCharacter (Pawn|GetControlledPawn)))
  (Default|ServerPlayMrIncredi _asthird_person_character (Class|KismetSystemLibrary|MakeLiteralInteger)))

(fn HandleMrIncredi2
  (bind _asthird_person_character (Utilities|Casting|CastToThirdPersonCharacter (Pawn|GetControlledPawn)))
  (Default|ServerPlayMrIncredi _asthird_person_character (Class|KismetSystemLibrary|MakeLiteralInteger 1)))

(fn HandleMrIncredi3
  (bind _asthird_person_character (Utilities|Casting|CastToThirdPersonCharacter (Pawn|GetControlledPawn)))
  (Default|ServerPlayMrIncredi _asthird_person_character (Class|KismetSystemLibrary|MakeLiteralInteger 2)))

(fn HandleSetPawnRelative3DScale
  (params (valueX :type Float%20%28single-precision%29) (valueY :type Float%20%28single-precision%29) (valueZ :type Float%20%28single-precision%29))
  (bind _asthird_person_character (Utilities|Casting|CastToThirdPersonCharacter (Pawn|GetControlledPawn)))
  (if (Variables|/Game/Player/ThirdPersonCharacter.ThirdPersonCharacter_C|GetbModsAllowed _asthird_person_character)
    (Default|ServerSetRelativeScale3d _asthird_person_character valueX valueY valueZ)
    (return)))

(fn HandleToggleModTools
  (bind _asthird_person_character (Utilities|Casting|CastToThirdPersonCharacter (Pawn|GetControlledPawn)))
  (if (Variables|/Game/Player/ThirdPersonCharacter.ThirdPersonCharacter_C|GetbModsAllowed _asthird_person_character)
    (Variables|/Game/Player/ThirdPersonCharacter.ThirdPersonCharacter_C|SetbModsAllowed _asthird_person_character false)
    (else
      (Variables|/Game/Player/ThirdPersonCharacter.ThirdPersonCharacter_C|SetbModsAllowed _asthird_person_character true)))
  (Default|OnModsToggled _asthird_person_character (Variables|/Game/Player/ThirdPersonCharacter.ThirdPersonCharacter_C|GetbModsAllowed _asthird_person_character)))

(fn HandleToggleSwitchViewTargetonFriendlyFire
  (bind _asthird_person_character (Utilities|Casting|CastToThirdPersonCharacter (Pawn|GetControlledPawn)))
  (Default|ServerToggleSwitchViewTargetonFF _asthird_person_character))

(fn HandleDisableInvisibilityfortheInnocent
  (bind _asthird_person_character (Utilities|Casting|CastToThirdPersonCharacter (Pawn|GetControlledPawn)))
  (Default|ServerDisableInvisibilityfortheInnocent _asthird_person_character))