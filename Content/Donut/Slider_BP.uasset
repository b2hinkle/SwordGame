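; Slider actor that acts as an animated sliding hazard, lethally damaging the third-person character when closed.
; Its skeletal mesh is driven by the Open flag on Sider_ANIMBP.
; Box overlap with the character's collision cylinder opens it briefly, then closes it.
; HitBox overlap with the character's capsule while closed calls DoDamage with a huge amount, then reopens it after a delay.
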(event OnComponentBeginOverlap(Box)
  (params (OverlappedComponent :type Primitive%20Component%20Object%20Reference) (OtherActor :type Actor%20Object%20Reference) (OtherComp :type Primitive%20Component%20Object%20Reference) (OtherBodyIndex :type Integer) (bFromSweep :type Boolean) (SweepResult :type Hit%20Result%20Structure%20%28by%20ref%29))
  (if (Utilities|Enum|Equal(Enum) (Utilities|GetObjectName OtherComp) "CollisionCylinder")
    (if (== (Utilities|GetClass OtherActor) "/Game/Player/ThirdPersonCharacter.ThirdPersonCharacter_C")
      (bind _assider_animbp (Utilities|Casting|CastToSider_ANIMBP (Components|SkeletalMesh|GetAnimInstance (Variables|Default|GetSkeletalMesh))))
      (Variables|/Game/Donut/Sider_ANIMBP.Sider_ANIMBP_C|SetbOpen _assider_animbp true)
      (Utilities|FlowControl|Delay 3.0)
      (Variables|/Game/Donut/Sider_ANIMBP.Sider_ANIMBP_C|SetbOpen _assider_animbp false))))

(event OnComponentBeginOverlap(HitBox)
  (params (OverlappedComponent :type Primitive%20Component%20Object%20Reference) (OtherActor :type Actor%20Object%20Reference) (OtherComp :type Primitive%20Component%20Object%20Reference) (OtherBodyIndex :type Integer) (bFromSweep :type Boolean) (SweepResult :type Hit%20Result%20Structure%20%28by%20ref%29))
  (if (== (Utilities|GetClass OtherComp) "/Script/Engine.CapsuleComponent")
    (bind _asthird_person_character (Utilities|Casting|CastToThirdPersonCharacter OtherActor))
    (bind _assider_animbp (Utilities|Casting|CastToSider_ANIMBP (Components|SkeletalMesh|GetAnimInstance (Variables|Default|GetSkeletalMesh))))
    (if (not (Variables|/Game/Donut/Sider_ANIMBP.Sider_ANIMBP_C|GetbOpen _assider_animbp))
      (Default|DoDamage _asthird_person_character 1e+03)
      (Utilities|FlowControl|Delay 3.5)
      (Variables|/Game/Donut/Sider_ANIMBP.Sider_ANIMBP_C|SetbOpen _assider_animbp true))))

(event EventBeginPlay)

(event Collision|EventActorBeginOverlap
  (params (OtherActor :type Actor%20Object%20Reference)))

(event EventTick
  (params (DeltaSeconds :type Float%20%28single-precision%29)))

(fn ConstructionScript)